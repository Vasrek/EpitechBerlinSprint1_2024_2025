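; Falling platform that drops after the player steps on it, then respawns at its starting spot.
; A box overlap from the player disarms it, steps the cube through orange and red warning materials with sounds, then enables physics.
; After a delay, it spawns a fresh copy at the location and rotation saved on BeginPlay and destroys itself.
; The older reset-in-place nodes are left unconnected.
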(event OnComponentBeginOverlap(Box)
  (params (OverlappedComponent :type Primitive%20Component%20Object%20Reference) (OtherActor :type Actor%20Object%20Reference) (OtherComp :type Primitive%20Component%20Object%20Reference) (OtherBodyIndex :type Integer) (bFromSweep :type Boolean) (SweepResult :type Hit%20Result%20Structure%20%28by%20ref%29))
  ;[0.06739 0.07008 1] Falling Platform
  ;;[1 1 1] Begin Overlap : Test if it's the player
  (if (and (== OtherActor (Game|GetPlayerCharacter 0)) (Variables|Default|GetIsActive?))
    ;;[1 1 1] first color change (orange)
    (Variables|Default|SetIsActive? false)
    (CallFunction|ChangeMaterialandPlaySound "/Engine/VREditor/Sounds/UI/Dockable_Window_Pick_Up.Dockable_Window_Pick_Up" "/Game/Materials/MI_Orange.MI_Orange")
    (Utilities|FlowControl|Delay 0.7)
    ;;[1 1 1] Second color change (red)
    (CallFunction|ChangeMaterialandPlaySound "/Engine/VREditor/Sounds/UI/Dockable_Window_Open.Dockable_Window_Open" "/Game/Materials/MI_Red.MI_Red")
    (Utilities|FlowControl|Delay 0.5)
    ;;[1 1 1] Enable physics
    (Physics|SetSimulatePhysics (Variables|Default|GetCube) true)
    (Audio|PlaySound2D "/Engine/VREditor/Sounds/UI/Drop_Item_From_ContentBrowser.Drop_Item_From_ContentBrowser" 1.0 1.0 0.0 0 0)
    ;;[1 1 1] Delay before respawn platform
    (Utilities|FlowControl|Delay 5.0)
    (CallFunction|RespawnPlatformtoDefaultLoc)))

(event Custom|ChangeMaterialAndPlaySound
  (params (Sound :type Sound%20Base%20Object%20Reference) (MaterialToSet :type Material%20Interface%20Object%20Reference))
  ;[0.06739 0.07008 1] Falling Platform
  ;;[1 1 1] Set material and play sfx
  (Rendering|Material|SetMaterial (Variables|Default|GetCube) 0 MaterialToSet)
  (Audio|PlaySound2D Sound 1.0 1.0 0.0 0 0))

(event Custom|RespawnPlatformToDefaultLoc
  (bind _defaultspawninfo (Variables|Default|GetDefaultSpawnInfo))
  ;[0.06739 0.07008 1] Falling Platform
  ;;[1 1 1] Disable physics / teleport platform to default transform / reset material
  (Game|SpawnActorfromClass "BP_FallingPlatform_C" (Math|Transform|MakeTransform (.location _defaultspawninfo) (.rotation _defaultspawninfo) "1.000000,1.000000,1.000000") "Undefined" "MultiplyWithRoot" 0 0)
  (Actor|DestroyActor))

(event EventBeginPlay
  ;[0.06739 0.07008 1] Falling Platform
  ;;[1 1 1] Save default transform
  (Variables|Default|SetDefaultSpawnInfo (Transformation|GetWorldTransform (Variables|Default|GetCube))))

(fn ConstructionScript)